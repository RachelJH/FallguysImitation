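; Trigger-driven obstacle Blueprint that breaks away three wall pieces when the player character reaches it.
; An overlap on the Box by BP_bwj_ThirdPersonCharacter turns on physics simulation for the left, right and D wall components.
; After a short delay, all three wall components are destroyed.
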(event `self.Box.OnComponentBeginOverlap`
  (params (OverlappedComponent :type "PrimitiveComponent Object Reference") (OtherActor :type "Actor Object Reference") (OtherComp :type "PrimitiveComponent Object Reference") (OtherBodyIndex :type Integer) (bFromSweep :type Boolean) (SweepResult :type "HitResult Structure (by ref)"))
  (bind _wall_l (`self.wall_l`))
  (bind _wall_r (`self.wall_r`))
  (bind _wall_d (`self.wall_d`))
  (cast `/Game/BWJ/bwj_thirdperson/BP_bwj_ThirdPersonCharacter` OtherActor)
  (`PrimitiveComponent.SetSimulatePhysics` _wall_l true)
  (`PrimitiveComponent.SetSimulatePhysics` _wall_r true)
  (`PrimitiveComponent.SetSimulatePhysics` _wall_d true)
  (`KismetSystemLibrary.Delay` 2.0)
  (`ActorComponent.K2_DestroyComponent` _wall_l)
  (`ActorComponent.K2_DestroyComponent` _wall_r)
  (`ActorComponent.K2_DestroyComponent` _wall_d))

(fn `UserConstructionScript`)
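; BP_FG_Characterloading is a character Blueprint for a multiplayer map, apparently a loading level, that displays its player's user name on a name tag widget.
; On BeginPlay it creates a WB_UserNameTag linked to itself and adds it to the viewport.
; It then binds to BP_LoadingPlayerState's name-change dispatcher and pushes the current name to the tag.
; If the player state cast fails, it prints a debug string and retries on a short timer.
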(event `self.ReceiveBeginPlay`
  (`self.CreateNameTag`))

(fn `BindPlayerState`
  (bind _asbp_loading_player_state (cast `/Game/SJH/Multiplayer/Level/Maps/Map1/BP_LoadingPlayerState` (`self.PlayerState`))
    (:`then`
      (add `/Game/SJH/Multiplayer/Level/Maps/Map1/BP_LoadingPlayerState.EventDispatcher_ChangeUeserName` _asbp_loading_player_state (`|CreateDelegate` :!event `UpdateUserName`))
      (`self.UpdateUserName` (`/Game/SJH/Multiplayer/Level/Maps/Map1/BP_LoadingPlayerState.UserName` _asbp_loading_player_state)))
    (:`CastFailed`
      (`KismetSystemLibrary.PrintString` "EventPlayerState" true true (struct :`G` 0.66 :`B` 1.0 :`A` 1.0) 33.0)
      (`KismetSystemLibrary.K2_SetTimer` null "BindPlayerState" 0.01))))

(fn `CreateNameTag`
  (bind _returnvalue (`|CreateWidget` "/Game/SJH/Multiplayer/Widgets/NameTag/WB_UserNameTag.WB_UserNameTag_C" null self))
  (bind _output_get (set `self.NameTag` _returnvalue))
  (`UserWidget.AddToViewport` _output_get 0)
  (`self.BindPlayerState`))

(fn `UpdateUserName`
  (params (UserName :type String))
  (`/Game/SJH/Multiplayer/Widgets/NameTag/WB_UserNameTag.UpdateNameTag` (`self.NameTag`) UserName))

(fn `UserConstructionScript`)
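; Player controller for the multiplayer loading map that reports player count and user name when it possesses a pawn.
; On the server, possession passes the game mode's player count and the GameInstance's max player count to the loading GameState.
; It then has the client read its user name from its GameInstance and send it back to the server, which updates the loading PlayerState.
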(event `self.ReceivePossess`
  (params (PossessedPawn :type "Pawn Object Reference"))
  ;[1 0 0] Server
  (`|ExecutionSequence`
    (:`then_0`
      (bind _returnvalue (`GameModeBase.GetNumPlayers` (`GameplayStatics.GetGameMode`)))
      (bind _asbp_loading_game_state (cast `/Game/SJH/Multiplayer/Level/Maps/LoadingMap/BP_LoadingGameState` (`GameplayStatics.GetGameState`)))
      (bind _asbp_game_instance (cast `/Game/SJH/Multiplayer/BP_GameInstance` (`GameplayStatics.GetGameInstance`)))
      (`/Game/SJH/Multiplayer/Level/Maps/LoadingMap/BP_LoadingGameState.UpdateUserCount` _asbp_loading_game_state _returnvalue (`/Game/SJH/Multiplayer/BP_GameInstance.MaxPlayerCount` _asbp_game_instance)))
    (:`then_1`
      (`self.GameUserName` PossessedPawn))))

(event `GameUserName`
  (params (Possess :type "Pawn Object Reference"))
  ;[1 1 1] Client
  (bind _asbp_game_instance (cast `/Game/SJH/Multiplayer/BP_GameInstance` (`GameplayStatics.GetGameInstance`)))
  (`self.ReqGameUserName` (`/Game/SJH/Multiplayer/BP_GameInstance.PlayerUserName` _asbp_game_instance)))

(event `ReqGameUserName`
  (params (UserName :type String))
  ;[1 0 0] Server
  (bind _asbp_loading_player_state (cast `/Game/SJH/Multiplayer/Level/Maps/LoadingMap/BP_LoadingPlayerState` (`self.PlayerState`)))
  (`/Game/SJH/Multiplayer/Level/Maps/LoadingMap/BP_LoadingPlayerState.UpdateUserName` _asbp_loading_player_state UserName))

(fn `UserConstructionScript`)
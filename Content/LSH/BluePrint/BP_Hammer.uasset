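; BP_Hammer is a spinning hammer obstacle that knocks the player character away on contact.
; Tick rolls its StaticMesh at a steady one revolution per second, scaled by delta time.
; A hit on the Box component by the first player's pawn casts it to BP_FG_Character and launches it along a fixed world Y direction.
; An unused calculation for position-based knockback remains unconnected.
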(event `self.ReceiveBeginPlay`)

(event `self.ReceiveTick`
  (params (DeltaSeconds :type "Float (single-precision)"))
  (`SceneComponent.K2_AddRelativeRotation` (`self.StaticMesh`) (`KismetMathLibrary.MakeRotator` (* DeltaSeconds -360.0)) false false))

(event `self.Box.OnComponentHit`
  (params (HitComponent :type "PrimitiveComponent Object Reference") (OtherActor :type "Actor Object Reference") (OtherComp :type "PrimitiveComponent Object Reference") (NormalImpulse :type "Vector Structure") (Hit :type "HitResult Structure (by ref)"))
  (bind _returnvalue (`GameplayStatics.GetPlayerPawn` 0))
  (if (== OtherActor _returnvalue)
    (bind _asbp_fg_character (cast `/Game/LSH/GameMode/BP_FG_Character` _returnvalue))
    (`Character.LaunchCharacter` _asbp_fg_character (0.0 500.0 0.0) false false)))

(fn `UserConstructionScript`)
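; Finish line actor that ends the match when an actor overlaps its box, showing the finish widget and treating a BP_FG_Character as the winner.
; CastFuncation records the winner in BP_GameInstance and triggers the controller's winner animation, returning inside its loop over player controllers.
; After a delay it streams in win_map, teleports the winner there, blends the first player's view to BP_Camera and calls BindWinnerPlayer.
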(event `self.ReceiveBeginPlay`)

(event `self.Box.OnComponentBeginOverlap`
  (params (OverlappedComponent :type "PrimitiveComponent Object Reference") (OtherActor :type "Actor Object Reference") (OtherComp :type "PrimitiveComponent Object Reference") (OtherBodyIndex :type Integer) (bFromSweep :type Boolean) (SweepResult :type "HitResult Structure (by ref)"))
  (`self.ShowWidget` OtherActor)
  (bind _outputpin (`self.CastFuncation` OtherActor))
  (`KismetSystemLibrary.Delay` 3.0)
  (`GameplayStatics.LoadStreamLevel` "win_map" true)
  (`self.K2_SetActorLocationAndRotation` _outputpin (-485.000926 19015.000024 150.0) (struct :`Yaw` -90.0) false false)
  (bind _returnvalue (`GameplayStatics.GetActorOfClass` "/Game/LSH/GameMode/GameFinish/BP_Camera.BP_Camera_C"))
  (bind _asbp_fg_contoller (cast `/Game/LSH/GameMode/BP_FG_Contoller` (`GameplayStatics.GetPlayerController` 0)))
  (`PlayerController.SetViewTargetWithBlend` _asbp_fg_contoller _returnvalue 1.0 "VTBlend_Linear" 0.0 false)
  (`/Game/LSH/GameMode/BP_FG_Character.BindWinnerPlayer` _outputpin))

(fn `CastFuncation`
  (params (InputPin :type "Object Object Reference"))
  (returns (OutputPin :type "/Game/LSH/GameMode/BP_FG_Character Object Reference"))
  (bind _outactors (`GameplayStatics.GetAllActorsOfClass` "/Script/Engine.PlayerController"))
  (for _array_element _outactors
    (`self.DisableInput` _array_element (`GameplayStatics.GetPlayerController` 0))
    (bind _asbp_fg_character (cast `/Game/LSH/GameMode/BP_FG_Character` InputPin))
    (bind _asbp_game_instance (cast `/Game/SJH/Multiplayer/BP_GameInstance` (`GameplayStatics.GetGameInstance`)))
    (`/Game/SJH/Multiplayer/BP_GameInstance.WinnerUser` _asbp_game_instance _asbp_fg_character)
    (bind _asbp_fg_contoller (cast `/Game/LSH/GameMode/BP_FG_Contoller` (`GameplayStatics.GetPlayerController` 0)))
    (`/Game/LSH/GameMode/BP_FG_Contoller.WinnerAnim` _asbp_fg_contoller _asbp_fg_character)
    (return _asbp_fg_character)))

(fn `ShowWidget`
  (params (Winner :type "Actor Object Reference"))
  (`self.DisableInput` Winner (`GameplayStatics.GetPlayerController` 0))
  (bind _returnvalue (`|CreateWidget` "/Game/LSH/GameMode/GameFinish/WB_Finish.WB_Finish_C"))
  (`UserWidget.AddToViewport` _returnvalue 0))

(fn `UserConstructionScript`)